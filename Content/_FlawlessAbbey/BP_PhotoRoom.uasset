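; Photo room Blueprint that lets the player inspect a mesh by rotating, zooming and resetting it through Enhanced Input.
; While IA_HoldView triggers, the negated IA_PanView value drives RotateMesh, and PanningDelta is zeroed.
; IA_Zoom and IA_Reset call ZoomMesh and ResetMesh, whose bodies are not defined here.
; IA_Look is empty, and the only write of input to PanningDelta is disconnected.
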(event Input|EnhancedActionEvents|EnhancedInputActionIA_Zoom
  (params (ActionValue :type Float%20%28double-precision%29) (ElapsedSeconds :type Float%20%28double-precision%29) (TriggeredSeconds :type Float%20%28double-precision%29) (InputAction :type Input%20Action%20Object%20Reference :default "/Game/_FlawlessAbbey/Input/IA_Zoom.IA_Zoom"))
  (Class|FAPhotoRoom|ZoomMesh ActionValue))

(event Input|EnhancedActionEvents|EnhancedInputActionIA_Look
  (params (ActionValue :type Vector%202D%20Structure) (ElapsedSeconds :type Float%20%28double-precision%29) (TriggeredSeconds :type Float%20%28double-precision%29) (InputAction :type Input%20Action%20Object%20Reference :default "/Game/FirstPerson/Input/Actions/IA_Look.IA_Look")))

(event Input|EnhancedActionEvents|EnhancedInputActionIA_Reset
  (params (ActionValue :type Boolean) (ElapsedSeconds :type Float%20%28double-precision%29) (TriggeredSeconds :type Float%20%28double-precision%29) (InputAction :type Input%20Action%20Object%20Reference :default "/Game/_FlawlessAbbey/Input/IA_Reset.IA_Reset"))
  (Class|FAPhotoRoom|ResetMesh))

(event Input|EnhancedActionEvents|EnhancedInputActionIA_HoldView
  (params (ActionValue :type Boolean) (ElapsedSeconds :type Float%20%28double-precision%29) (TriggeredSeconds :type Float%20%28double-precision%29) (InputAction :type Input%20Action%20Object%20Reference :default "/Game/_FlawlessAbbey/Input/IA_HoldView.IA_HoldView"))
  (bind _returnvalue (Input|EnhancedActionValues|GetIA_PanView))
  (Class|FAPhotoRoom|RotateMesh (Math|Vector2D|MakeVector2D (* (.x _returnvalue) -1.0) (* (.y _returnvalue) -1.0)))
  (Variables|Default|SetPanningDelta ""))

(event EventBeginPlay)

(event Collision|EventActorBeginOverlap
  (params (OtherActor :type Actor%20Object%20Reference)))

(event EventTick
  (params (DeltaSeconds :type Float%20%28single-precision%29)))

(fn ConstructionScript)